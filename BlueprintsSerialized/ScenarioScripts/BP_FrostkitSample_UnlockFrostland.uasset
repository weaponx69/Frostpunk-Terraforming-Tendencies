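; BP_FrostkitSample_UnlockFrostland is a sample scenario script that opens up the Frostland once a logistics district is built.
; On BeginPlay it binds to the construction subsystem's finished event.
; When a finished construction's owner has a district component and the Logistics tag, it activates the Frostland-available context and unlocks the first-logistics-built asset for the player nation.
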(event `self.ReceiveBeginPlay`
  (add `PXConstructionSubsystem.ConstructionFinishedEvent` (subsystem `PXConstructionSubsystem`) (delegate `OnConstructionFinished`)))

(event `OnConstructionFinished`
  (params (constructionComponent :type "PXConstructionComponent Object Reference"))
  (bind _output_get (set `self.District` (`Actor.GetComponentByClass` (`ActorComponent.GetOwner` constructionComponent) "/Script/Frostpunk2.PXDistrictComponent")))
  (`/Engine/EditorBlueprintResources/StandardMacros.IsValid` _output_get
    (:`Is Valid`
      (if (`PXTagUtils.HasGameplayTag` (`ActorComponent.GetOwner` (`self.District`)) (struct :`TagName` "District.Logistics"))
        (`PXContextUtils.SetContextActive` "/Game/Scenarios/Shared/Configs/Contexts/Simple/DA_FrostlandAvailableContext.DA_FrostlandAvailableContext" true)
        (`PXUnlockUtils.SetUnlockActive` (`PXNationUtils.GetPlayerNation`) "/Game/Scenarios/Shared/Configs/Unlocks/Other/DA_FirstLogisticBuilt.DA_FirstLogisticBuilt" true)))))