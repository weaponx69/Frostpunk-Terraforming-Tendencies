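; BP_FrostkitSample_VariableStorage is a variable storage Blueprint for the Frostkit sample, exposing story choices, endings and endlog data.
; Most story getters return fixed defaults or empty values instead of stored state.
; Endlog facts and chapter dates are written to and read from maps.
; Policies used in the log, pre-Oil Age ranked policies and the legacy faction are read from variables.
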(fn `Get Chapter Start Date`
  (params (Key :type "/Game/Scenarios/Shared/BlueprintsNonSerialized/PrimaryDataAssets/BP_EndlogFact_Config Object Reference"))
  (returns (Value :type "PXGameTime Structure"))
  (return (`BlueprintMapLibrary.Map_Find` (`self.Chapter Dates`) Key)))

(fn `Get Chosen Utopia`
  (returns (ChosenUtopia :type "/Game/Scenarios/Main/BlueprintsNonSerialized/ScenarioFunctionLibrary/ENUM_S1_UtopiaChoice Enum"))
  (return "NewEnumerator2"))

(fn `Get Faction War Ending`
  (returns (FactionWarEnding :type "/Game/Scenarios/Main/BlueprintsNonSerialized/Enums/ENUM_S1_FactionWarEnding Enum"))
  (return "NewEnumerator0"))

(fn `Get Faction War Strategy Choice`
  (returns (FactionWarPathChoice :type "/Game/Scenarios/Shared/BlueprintsSerialized/VariableStorage/ENUM_FactionWarStrategyChoice Enum"))
  (return "NewEnumerator0"))

(fn `Get Gas Toxicity`
  (returns (GasToxicity :type Integer))
  (return 0))

(fn `Get Heat Surplus Defeated`
  (returns (HeatSurplusDefeated :type Integer))
  (return 0))

(fn `Get Legacy Faction`
  (returns (`Legacy Faction` :type "/Game/Scenarios/Main/BlueprintsNonSerialized/Enums/VariableStorage/ENUM_LegacyFaction Enum"))
  (return (`self.Legacy Faction`)))

(fn `Get Next Gas Outburst Timestamp`
  (returns (NextGasOutburstTime :type "PXGameTime Structure"))
  (return))

(fn `Get Nomads Bell Tolls`
  (returns (`Nomads Bell Toll Count` :type Integer))
  (return 0))

(fn `Get Nomads Cemetery`
  (returns (NomadsCemetary :type "/Game/Scenarios/Main/BlueprintsNonSerialized/Enums/ENUM_S1_Nomadscemetery Enum"))
  (return "NewEnumerator0"))

(fn `Get Nomads Ending`
  (returns (`Nomads Ending` :type "/Game/Scenarios/Main/BlueprintsNonSerialized/Enums/VariableStorage/ENUM_NomadsEnding Enum"))
  (return "NewEnumerator3"))

(fn `Get Ranked Polices Before Oil Age Lens for Endlog`
  (returns (`Ranked Policies Before Oil Age Lens` :type "Array of PXPolicyType Object Reference"))
  (return (`self.Ranked Policies Before Oil Age Lens`)))

(fn `Get Settlements Embraced`
  (returns (SettlementsEmbraced :type Integer))
  (return 0))

(fn `Get Wanderers Camp Promise`
  (returns (`Wanderers Camp Promise` :type "/Game/Scenarios/Main/BlueprintsNonSerialized/ScenarioFunctionLibrary/ENUM_S1_WanderersCampPromise Enum"))
  (return "NewEnumerator0"))

(fn `Get Whiteout Incident Choice`
  (returns (`Whiteout Incident Choice` :type "/Game/Scenarios/Main/BlueprintsNonSerialized/ScenarioFunctionLibrary/ENUM_S1_WhiteoutIncidentChoice Enum"))
  (return "NewEnumerator0"))

(fn `Get Whiteout Timestamp`
  (returns (WhiteoutTimestamp :type "PXGameTime Structure"))
  (return))

(fn `Get Winterhome Choice`
  (returns (WinterhomeChoice :type "/Game/Scenarios/Main/BlueprintsNonSerialized/ScenarioFunctionLibrary/ENUM_S1_WinterhomeChoice Enum"))
  (return "NewEnumerator2"))

(fn `Get Winterhome Cores`
  (returns (WinterhomeCoresObjectiveFinished :type Boolean))
  (return false))

(fn `Is Fact Logged?`
  (params (ItemToFind :type "/Game/Scenarios/Shared/BlueprintsNonSerialized/PrimaryDataAssets/BP_EndlogFact_Config Object Reference"))
  (returns (`Is Logged?` :type Boolean) (`Formatted Text` :type Text))
  (bind (_value _returnvalue) (`BlueprintMapLibrary.Map_Find` (`self.Logged Endlog Facts`) ItemToFind))
  (if (`KismetSystemLibrary.IsValid` ItemToFind)
    (return _returnvalue _value)
    (else
      (return false ""))))

(fn `Is Policy Used in Log?`
  (params (ItemToFind :type "PXPolicyType Object Reference (by ref)"))
  (returns (ReturnValue :type Boolean))
  (return (`KismetArrayLibrary.Array_Contains` (`self.Policies Used in Log`) ItemToFind)))

(fn `Log Chapter Date`
  (params (Key :type "/Game/Scenarios/Shared/BlueprintsNonSerialized/PrimaryDataAssets/BP_EndlogFact_Config Object Reference") (Value :type "PXGameTime Structure"))
  (`BlueprintMapLibrary.Map_Add` (`self.Chapter Dates`) Key Value))

(fn `Log Endlog Fact`
  (params (`Item to Log` :type "/Game/Scenarios/Shared/BlueprintsNonSerialized/PrimaryDataAssets/BP_EndlogFact_Config Object Reference") (`Formatted Text` :type Text))
  (`BlueprintMapLibrary.Map_Add` (`self.Logged Endlog Facts`) `Item to Log` `Formatted Text`))