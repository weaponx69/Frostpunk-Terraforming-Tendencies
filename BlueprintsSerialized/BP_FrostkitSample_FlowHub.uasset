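; Flow hub for the Frostkit sample scenario, scripting its opening and quest chain from BeginPlay.
; After an intro chorister message and opening cutscene, it activates the city view, unlocks Hall of Delegates and Research Institute, and sets up New London's communities, faction and absence modifier.
; A sequence then chains the Coal and Basics quests, each preceded by a dialog, into an end message, and also deactivates generator logic.
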(event `self.ReceiveBeginPlay`
  (bind _returnvalue (`PXNationUtils.GetPlayerNation`))
  (`PXAsyncWaitForLoadingScreenFadedOut.AsyncAction_WaitForLoadingScreenFadedOut`
    (:`Completed`
      (bind _decision (`/Game/Scenarios/Shared/BlueprintsNonSerialized/SocietyUtils/BPFL_Communication_Utils.Send Config Message` "/Game/Scenarios/FrostkitSampleScenario/Configs/Messages/Choristers/DA_FrostkitSample_Intro_Chorister.DA_FrostkitSample_Intro_Chorister" null null null (`|MakeMap` "" :!valuetype "Text") null null (struct) true))
      (`PXAsyncWaitForAnyChoice.AsyncAction_WaitForAnyChoice` _decision
        (:`Completed`
          (`PXPlayerContextUtils.StartCameraCutscene` "/Game/Scenarios/FrostkitSampleScenario/Configs/PlayerContext/OpeningCutscene.OpeningCutscene")
          (`PXAsyncWaitForCutsceneEnd.AsyncAction_WaitForCutsceneEnd` "/Game/Scenarios/FrostkitSampleScenario/Configs/PlayerContext/OpeningCutscene.OpeningCutscene"
            (:`Completed`
              (`PXContextUtils.SetContextActive` "/Game/Scenarios/Shared/Configs/Contexts/Simple/DA_CityViewContext.DA_CityViewContext" true)
              (set `self.Main City Component` (`PXCityUtils.GetCityByType` "/Game/Scenarios/FrostkitSampleScenario/Configs/DA_FrostkiSample_City_EdensPoint_Startup.DA_FrostkiSample_City_EdensPoint_Startup"))
              (`PXUnlockUtils.SetUnlockActive` _returnvalue "/Game/Scenarios/Shared/Configs/Unlocks/DA_HoDUnlocked.DA_HoDUnlocked" true)
              (`PXUnlockUtils.SetUnlockActive` _returnvalue "/Game/Scenarios/Shared/Configs/Unlocks/DA_ResearchInstituteUnlocked.DA_ResearchInstituteUnlocked" true)
              (`PXCommunityUtils.ChangeCommunitySize` 2500 (make `PXCommunitySizeChangeParameters` "Growth" (`self.Main City Component`) "/Game/Scenarios/Main/Configs/Communities/CommunityTypes/DA_NewLondoners_NLScenario.DA_NewLondoners_NLScenario" "starting community"))
              (`PXCommunityUtils.ChangeCommunitySize` 1000 (make `PXCommunitySizeChangeParameters` "Growth" (`self.Main City Component`) "/Game/Scenarios/Main/Configs/Communities/CommunityTypes/DA_CommunityOrder_NLScenario.DA_CommunityOrder_NLScenario" "starting community"))
              (`PXCommunityUtils.ChangeCommunitySize` 2500 (make `PXCommunitySizeChangeParameters` "Growth" (`self.Main City Component`) "/Game/Scenarios/Main/Configs/Communities/CommunityTypes/DA_Frostlanders_NLScenario.DA_Frostlanders_NLScenario" "starting community"))
              (`PXFactionUtils.FormFaction` "/Game/Scenarios/Main/Configs/Factions/M3Factions/DA_FactionOrder.DA_FactionOrder")
              (`/Game/Scenarios/Shared/BlueprintsNonSerialized/FactionEmergence/BPFL_FactionEmergenceUtils.Set Community Trust` 0.0)
              (`PXCommunityUtils.AddImprint` (`.ReturnValue` (`PXCommunityUtils.GetCommunityOfCommunityType` "/Game/Scenarios/Main/Configs/Communities/CommunityTypes/DA_CommunityOrder_NLScenario.DA_CommunityOrder_NLScenario")) "/Game/Scenarios/Main/Configs/Communities/Imprints/Other/DA_NL_StartingFaction_Loyalty.DA_NL_StartingFaction_Loyalty")
              (`/Game/Scenarios/Shared/BlueprintsNonSerialized/SocietyUtils/BPFL_Communication_Utils.Refresh Global Text Tags`)
              (`/Game/Scenarios/Shared/BlueprintsNonSerialized/SocietyUtils/BPFL_StoryArc_Utils.Set PeoplesVoices activity` true)
              (`PXVoiceOverCoordinatorUtils.RemoveAllVoiceOversBlockReason` "/Game/Scenarios/Shared/Configs/VoiceOver/BlockReasons/DA_VoiceOverDefaultBlockReason.DA_VoiceOverDefaultBlockReason")
              (`self.Set Absence Modifier`)
              (`|ExecutionSequence`
                (:`then_0`
                  (bind _selectedchoiceindex (`PXAsyncOpenPredefinedDialog.AsyncAction_OpenPredefinedDialog` "/Game/Scenarios/FrostkitSampleScenario/Configs/Messages/Dialogs/DA_FrostkitSample_ProvideCoal.DA_FrostkitSample_ProvideCoal")
                    (:`Completed`
                      (switch `int` (`KismetMathLibrary.Conv_ByteToInt` _selectedchoiceindex)
                        (:`Default`
                          (bind _returnvalue_2 (`PXQuestUtils.StartQuest` "/Game/Scenarios/FrostkitSampleScenario/BlueprintsSerialized/Quests/BP_FrostkitSample_Coal.BP_FrostkitSample_Coal_C"))
                          (bind _succeeded (`PXAsyncWaitForQuest.AsyncAction_WaitForQuest` _returnvalue_2)
                            (:`Completed`
                              (if _succeeded
                                (bind _selectedchoiceindex_2 (`PXAsyncOpenPredefinedDialog.AsyncAction_OpenPredefinedDialog` "/Game/Scenarios/FrostkitSampleScenario/Configs/Messages/Dialogs/DA_FrostkitSample_BasicsMessage.DA_FrostkitSample_BasicsMessage")
                                  (:`Completed`
                                    (switch `int` (`KismetMathLibrary.Conv_ByteToInt` _selectedchoiceindex_2)
                                      (:`Default`
                                        (bind _returnvalue_3 (`PXQuestUtils.StartQuest` "/Game/Scenarios/FrostkitSampleScenario/BlueprintsSerialized/Quests/BP_FrostkitSample_Basics.BP_FrostkitSample_Basics_C"))
                                        (bind _succeeded_2 (`PXAsyncWaitForQuest.AsyncAction_WaitForQuest` _returnvalue_3)
                                          (:`Completed`
                                            (if _succeeded_2
                                              (`PXAsyncOpenPredefinedDialog.AsyncAction_OpenPredefinedDialog` "/Game/Scenarios/FrostkitSampleScenario/Configs/Messages/Dialogs/DA_FrostkitSample_EndMessage.DA_FrostkitSample_EndMessage"))))))))))))))))
                (:`then_1`
                  (`PXActivityUtils.DeactivateLogic` (`ActorComponent.GetOwner` (`PXGeneratorUtils.GetGeneratorFromCity` (`self.Main City Component`))) "/Game/Scenarios/Shared/Configs/Activity/DeactivationTypes/DA_DeactivationReason_GeneratorAfterIntro_NL.DA_DeactivationReason_GeneratorAfterIntro_NL"))))))))))

(fn `Check Skip Cutscene`
  (returns (ReturnValue :type Boolean))
  (return false))

(fn `Set Absence Modifier`
  (`PXPredefinedModifierUtils.SetPredefinedModifierActive` (`PXNationUtils.GetPlayerNation`) (`/Game/Scenarios/Main/Configs/Constants/BP_S1_Constants_BaseClass.NLStartingAbsenceModifiers` (`/Game/Scenarios/Main/BlueprintsNonSerialized/ScenarioFunctionLibrary/BPFL_S1_ScenarioStorage.Get S1 Constants Storage`)) true))