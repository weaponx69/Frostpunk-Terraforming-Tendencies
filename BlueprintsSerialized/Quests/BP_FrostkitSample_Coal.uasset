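; Sample Frostkit quest that tasks the player with Frostbreaking to a coal deposit and building an Extraction District there.
; On start it registers a tagged-district build objective limited to tiny or deep coal deposits, then blocks background chatter.
; After a timed async wait, it resolves the main district's hub and, if valid, plays a 3D voice line there and lifts the chatter block.
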(event `self.ReceiveStartQuest`
  (`self.Initialize Objectives`)
  (`PXVoiceOverCoordinatorUtils.AddBackgroundChatterBlockReason` "/Game/Scenarios/FrostkitSampleScenario/Configs/BlockReasons/DA_FrostkitSampleImportant_Block.DA_FrostkitSampleImportant_Block")
  (`PXAsyncWaitForDurationPassed.AsyncAction_WaitForDurationPassed` (struct :`ScaledTicks` 720)
    (:`Completed`
      (bind _returnvalue (`PXDistrictUtils.ResolveHubFromBaseDistrict` (`PXCityComponent.GetMainDistrict` (`PXNationUtils.GetPlayerMainCity`)))
        (:`ComponentIsValid`
          (`/Game/Scenarios/Shared/BlueprintsNonSerialized/Audio/BPFL_AudioUtils.Post 3d Audio Event` "/Game/Scenarios/Shared/Audio/Events/VO/Background_Chatters/VO_MALE_01_CHAT_H_TRUST_3_PA.VO_MALE_01_CHAT_H_TRUST_3_PA" _returnvalue)
          (`PXVoiceOverCoordinatorUtils.RemoveBackgroundChatterBlockReason` "/Game/Scenarios/FrostkitSampleScenario/Configs/BlockReasons/DA_FrostkitSampleImportant_Block.DA_FrostkitSampleImportant_Block"))))))

(fn `Initialize Objectives`
  (bind _returnvalue (`PXQuestUtils.AddDistrictWithTagsQuestObjective` (make `PXObjectiveParameters` "Frostbreak to a Shallow Coal Seam and construct an Extraction District" "" false 1 false null self) (make `PXDistrictWithTagsObjectiveParameters` "Build" (struct :`TagName` "District.Extraction") 1 (`|MakeArray` "/Game/Scenarios/Shared/Configs/Deposits/DepositTypes/Coal/DA_Deposit_Coal_Tiny.DA_Deposit_Coal_Tiny" "/Game/Scenarios/Shared/Configs/Deposits/DepositTypes/Coal/DeepDeposits/DA_DeepDeposit_Coal.DA_DeepDeposit_Coal" :!type "PXDepositType Object Reference"))))
  (set `self.ExtractionObjective` _returnvalue))