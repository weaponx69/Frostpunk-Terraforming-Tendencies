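; Sample FrostKit quest for basic New London tasks: turning on the Central District Generator and building two Housing Districts.
; StartQuest creates both objectives, blocks background chatter and listens for generator changes; an active default Generator completes its objective.
; On completion it unbinds, waits, then plays a 3D voice line at the main district's hub and lifts the chatter block.
; A coal Extraction District objective exists but is unconnected.
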(event `self.ReceiveStartQuest`
  (`self.Initialize Objectives`)
  (`PXVoiceOverCoordinatorUtils.AddBackgroundChatterBlockReason` "/Game/Scenarios/Terraforming-Tendencies/Configs/BlockReasons/DA_FrostkitSampleImportant_Block.DA_FrostkitSampleImportant_Block")
  (add `PXGeneratorSubsystem.GeneratorChangedEvent` (`|Subsystem`) (delegate `GeneratorObjectiveProgress`)))

(event `GeneratorObjectiveProgress`
  (params (generator :type "PXGeneratorComponent Object Reference") (reason :type "EPXGeneratorChangeReason Enum" :default "Updated"))
  (bind _returnvalue_passed (break `PXCheckResult` (`PXActivityUtils.IsLogicActive` (`ActorComponent.GetOwner` generator))))
  (if (== (`PXGeneratorComponent.GetType` generator) "/Game/Scenarios/Shared/Configs/Generator/GeneratorTypes/DA_DefaultGenerator.DA_DefaultGenerator")
    (if _returnvalue_passed
      (`PXQuestObjective.ProgressObjective` (`self.GeneratorObjective`) 1
        (:`Finished`
          (remove `PXGeneratorSubsystem.GeneratorChangedEvent` (`|Subsystem`) (delegate `GeneratorObjectiveProgress`))
          (`PXAsyncWaitForDurationPassed.AsyncAction_WaitForDurationPassed` (struct :`ScaledTicks` 720)
            (:`Completed`
              (bind _returnvalue (`PXDistrictUtils.ResolveHubFromBaseDistrict` (`PXCityComponent.GetMainDistrict` (`PXNationUtils.GetPlayerMainCity`)))
                (:`ComponentIsValid`
                  (`/Game/Scenarios/Shared/BlueprintsNonSerialized/Audio/BPFL_AudioUtils.Post 3d Audio Event` "/Game/Scenarios/Shared/Audio/Events/VO/Background_Chatters/VO_MALE_01_CHAT_H_TRUST_3_PA.VO_MALE_01_CHAT_H_TRUST_3_PA" _returnvalue)
                  (`PXVoiceOverCoordinatorUtils.RemoveBackgroundChatterBlockReason` "/Game/Scenarios/Terraforming-Tendencies/Configs/BlockReasons/DA_FrostkitSampleImportant_Block.DA_FrostkitSampleImportant_Block"))))))))))

(fn `Initialize Objectives`
  (bind _returnvalue (`self.AddQuestObjective` "Turn on the Generator in Central District of New London" "" 0 1 false null "DebugObjectiveName" false (struct)))
  (set `self.GeneratorObjective` _returnvalue)
  (bind _returnvalue_2 (`PXQuestUtils.AddDistrictWithTagsQuestObjective` (make `PXObjectiveParameters` "Construct new Housing Districts to address lack of shelter" "" false 1 false null self) (make `PXDistrictWithTagsObjectiveParameters` "Build" (struct :`TagName` "District.Housing") 2)))
  (set `self.HousingObjective` _returnvalue_2))